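; Bomb actor whose Explode event spawns a scaled explosion particle and sound, then breaks and scatters Chaos physics objects.
; A FieldSystemComponent applies external cluster strain through a radial falloff sized and centred on the Sphere component.
; It then applies linear velocity from a radial vector, culled outside that same radius to confine the outward push to the blast sphere.
; Nothing in this Blueprint calls Explode itself.
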(event Custom|Explode
  (bind _returnvalue (Transformation|GetActorLocation))
  (bind _fieldsystemcomponent (Variables|Field|GetFieldSystemComponent))
  (bind _radialfalloff (Variables|Default|GetRadialFalloff))
  (bind _sphere (Variables|Default|GetSphere))
  (bind _returnvalue_2 (Components|Sphere|GetScaledSphereRadius _sphere))
  (bind _returnvalue_3 (Transformation|GetWorldLocation _sphere))
  (bind _returnvalue_4 (Field|SetRadialFalloff _radialfalloff 5e+05 0.0 1.0 0.0 _returnvalue_2 _returnvalue_3 "Field_FallOff_None"))
  (Effects|SpawnEmitteratLocation "/Game/StarterContent/Particles/P_Explosion.P_Explosion" _returnvalue "0, 0, 0" "3.000000,3.000000,3.000000")
  (Audio|PlaySoundatLocation "/Game/StarterContent/Audio/Explosion_Cue.Explosion_Cue" _returnvalue "0, 0, 0" 1.0 1.0 0.0 0 0 0 0)
  (Class|FieldSystemComponent|ApplyPhysicsField _fieldsystemcomponent true "Field_ExternalClusterStrain" 0 _returnvalue_4)
  (Class|FieldSystemComponent|ApplyPhysicsField _fieldsystemcomponent true "Field_LinearVelocity" 0 (Field|SetCullingField (Variables|Default|GetCullingField) _returnvalue_4 (Field|SetRadialVector (Variables|Default|GetRadialVector) 1e+03 _returnvalue_3) "Field_Culling_Outside")))

(fn ConstructionScript)